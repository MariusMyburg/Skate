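; BP_PhysicsSkater is a physics-driven skateboard actor that pushes itself along continuously, with no input handling in its graph.
; Each tick it snaps the Scene component to the skateboard mesh's world location and rotation, without sweep or teleport.
; It then applies a constant-magnitude force to the skateboard's root bone along the Arrow component's forward vector.
; BeginPlay, overlap and construction logic are empty.
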(event EventBeginPlay)

(event Collision|EventActorBeginOverlap
  (params (OtherActor :type Actor%20Object%20Reference)))

(event EventTick
  (params (DeltaSeconds :type Float%20%28single-precision%29))
  (bind _scene (Variables|Default|GetScene))
  (bind _sk_skateboard (Variables|Default|GetSK_Skateboard))
  (Transformation|SetWorldLocation _scene (Transformation|GetWorldLocation _sk_skateboard) false false)
  (Transformation|SetWorldRotation _scene (Transformation|GetWorldRotation _sk_skateboard) false false)
  (Physics|AddForce (Variables|Default|GetSK_Skateboard) (* (Math|Vector|GetForwardVector (Variables|Default|GetArrow)) 2e+04) "skateboard_rootnode" false))

(fn ConstructionScript)