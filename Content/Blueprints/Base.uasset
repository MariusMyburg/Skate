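; Base is a skateboard actor that simulates physics in the world until it is used.
; An overlap sphere registers the board on an overlapping Skater as its Skateboard reference, and end overlap leaves that reference in place.
; The onUsed event disables physics and collision and hides the widget, while onLeft restores all three.
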(event OnComponentBeginOverlap(Sphere)
  (params (OverlappedComponent :type Primitive%20Component%20Object%20Reference) (OtherActor :type Actor%20Object%20Reference) (OtherComp :type Primitive%20Component%20Object%20Reference) (OtherBodyIndex :type Integer) (bFromSweep :type Boolean) (SweepResult :type Hit%20Result%20Structure%20%28by%20ref%29))
  ;[1 1 1] Comment
  (bind _asskater (Utilities|Casting|CastToSkater OtherActor))
  (Variables|/Game/Blueprints/Skater.Skater_C|Setskateboard _asskater self))

(event OnComponentEndOverlap(Sphere)
  (params (OverlappedComponent :type Primitive%20Component%20Object%20Reference) (OtherActor :type Actor%20Object%20Reference) (OtherComp :type Primitive%20Component%20Object%20Reference) (OtherBodyIndex :type Integer))
  ;[1 1 1] Comment
)

(event Custom|onUsed
  ;[1 1 1] Comment
  (Physics|SetSimulatePhysics (Variables|Default|Getskateboard_base1) false)
  (Collision|SetCollisionEnabled (Variables|Default|Getskateboard_base1) "NoCollision")
  (Rendering|SetVisibility (Variables|Default|GetWidget) false false))

(event Custom|onLeft
  ;[1 1 1] Comment
  (Physics|SetSimulatePhysics (Variables|Default|Getskateboard_base1) true)
  (Collision|SetCollisionEnabled (Variables|Default|Getskateboard_base1) "QueryAndPhysics")
  (Rendering|SetVisibility (Variables|Default|GetWidget) true false))

(event EventBeginPlay
  ;[1 1 1] Comment
  (if (not (Variables|Default|Getused))
    (Physics|SetSimulatePhysics (Variables|Default|Getskateboard_base1) true)))

(fn ConstructionScript)