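; Player skater character that walks, runs and rides a skateboard, swapping between CharacterMovement and FloatingPawnMovement.
; While skating, Tick traces the ground to align the capsule, applies slope to speed, and hand-builds velocity for ollies, vert and air gravity.
; Input drives steering, camera and AnimBP flags, while Pushing and OlieFunction events apply pushes and jumps.
; Falling drops the board and ragdolls from the hip, with the capsule following until stand-up.
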(event EventPushing
  (params (out :type Boolean))
  ;[1 1 1] Skate Input
  (if out
    (Variables|/Game/Blueprints/SkatingBlueprint.SkatingBlueprint_C|Setpush (Variables|Default|GetanimBP) false)
    (else
      (Variables|Default|Setspeed (+ (Variables|Default|Getspeed) 2.5e+02)))))

(event EventBeginPlay
  ;[1 1 1] TICK
  ;;[1 1 1] Init
  (Utilities|FlowControl|Sequence
    (:then_0
      (bind _asskating_blueprint (Utilities|Casting|CastToSkatingBlueprint (Components|SkeletalMesh|GetAnimInstance (Variables|Character|GetMesh))))
      (Variables|Default|SetanimBP _asskating_blueprint)
      (Variables|Default|Setscore 200)
      (Variables|/Game/Blueprints/SkatingBlueprint.SkatingBlueprint_C|Setskating (Variables|Default|GetanimBP) (Variables|Default|Getskating)))
    (:then_1
      (if (Variables|Default|Getskating)
        (CallFunction|SpawnSkateboard)
        (Components|Activation|SetActive (Variables|Default|GetFloatingPawnMovement) true false)
        (Components|Activation|Deactivate (Variables|Character|GetCharacterMovement))
        (else
          (Components|Activation|SetActive (Variables|Character|GetCharacterMovement) true false)
          (Components|Activation|Deactivate (Variables|Default|GetFloatingPawnMovement)))))))

(event EventOlieFunction
  (params (end :type Boolean))
  ;[1 1 1] TICK
  ;;[1 1 1] Olie
  (Variables|Default|Setolie_up true))

(event EventTick
  (params (DeltaSeconds :type Float%20%28single-precision%29))
  (bind _surfacenormal (Variables|Default|GetsurfaceNormal))
  (bind _capsulecomponent (Variables|Default|GetCapsuleComponent))
  (bind _returnvalue (Math|Vector|GetRightVector _capsulecomponent))
  (bind _returnvalue_2 (Class|KismetMathLibrary|MakeRotfromYZ _returnvalue _surfacenormal))
  (bind _pitch (Math|Rotator|BreakRotator _returnvalue_2))
  ;[1 1 1] TICK
  ;;[1 1 1] Comment
  (Variables|Default|Setdelta DeltaSeconds)
  (CallFunction|ZoomCamera)
  (if (Variables|Default|Getskating)
    (CallFunction|TraceGround)
    (CallFunction|TraceBoard)
    (if (or (Variables|Default|GetinAir) (Variables|Default|Getolie_up))
      (if (and (Variables|Default|Getolie_up) (> (Math|Float|Absolute(Float) (Variables|Default|GetairRotation)) 1e+01))
        (Variables|Default|Setspeed (select (> (Variables|Default|Getspeed) 0.0) (* (Math|Float|Absolute(Float) (Variables|Default|Getspeed)) -1.0) (Math|Float|Absolute(Float) (Variables|Default|Getspeed)))))
      (Variables|/Game/Blueprints/SkatingBlueprint.SkatingBlueprint_C|SetinAir (Variables|Default|GetanimBP) true)
      (CallFunction|TraceLedge)
      (if (Variables|Default|Getolie_up)
        ;;[1 1 1] Olie
        (bind _distance (CallFunction|GetGroundDistance))
        (if (> _distance 1.2e+02)
          (Variables|Default|Setolie_up false)
          (else
            (bind _output_get (Variables|Default|SetAddVelocity (+ "0, 0,10.000000" (Variables|Default|GetAddVelocity))))
            (Variables|/Script/Engine.MovementComponent|SetVelocity (Variables|Default|GetFloatingPawnMovement) _output_get)))
        (elif (<= (.Pitch (Math|Rotator|BreakRotator (Math|Conversions|RotationFromXVector (Variables|Default|GetsurfaceNormal)))) 5e+01)
          ;;[1 1 1] Vert
          (bind _output_get_2 (Variables|Default|SetAddVelocity (Math|Vector|ProjectVectorontoPlane (+ "0, 0,-9.800000" (Variables|Default|GetAddVelocity)) (Variables|Default|GetsurfaceNormal))))
          (Variables|/Script/Engine.MovementComponent|SetVelocity (Variables|Default|GetFloatingPawnMovement) _output_get_2)
          (|CorrectSpeed)
          (else
            ;;[1 1 1] Air
            (bind _output_get_3 (Variables|Default|SetAddVelocity (+ "0, 0,-9.800000" (Variables|Default|GetAddVelocity))))
            (Variables|/Script/Engine.MovementComponent|SetVelocity (Variables|Default|GetFloatingPawnMovement) _output_get_3))))
      (else
        (Variables|/Game/Blueprints/SkatingBlueprint.SkatingBlueprint_C|SetinAir (Variables|Default|GetanimBP) false)
        (Transformation|SetWorldRotation (Variables|Default|GetCapsuleComponent) (Math|Rotator|MakeRotator (.Roll (Math|Rotator|BreakRotator (Math|Rotator|MakeRotfromXZ (Math|Vector|GetForwardVector (Variables|Default|GetCapsuleComponent)) _surfacenormal))) _pitch (.Yaw (Math|Rotator|BreakRotator (Transformation|GetWorldRotation _capsulecomponent)))) false false)
        (Variables|Default|Setspeed (- (Variables|Default|Getspeed) (/ _pitch 9.8)))
        (bind _output_get_4 (Variables|Default|SetAddVelocity (* (Math|Vector|GetForwardVector (Variables|Default|GetCapsuleComponent)) (Variables|Default|Getspeed))))
        (Variables|/Script/Engine.MovementComponent|SetVelocity (Variables|Default|GetFloatingPawnMovement) _output_get_4)))
    (else
      (Utilities|FlowControl|Sequence
        (:then_0
          (if (Variables|Default|Getragdoll)
            (CallFunction|CorrectRagdoll)
            (else
              (CallFunction|StandUpRagdoll))))))))

(event Collision|EventHit
  (params (MyComp :type Primitive%20Component%20Object%20Reference) (Other :type Actor%20Object%20Reference) (OtherComp :type Primitive%20Component%20Object%20Reference) (bSelfMoved :type Boolean) (HitLocation :type Vector :default "0, 0, 0") (HitNormal :type Vector :default "0, 0, 0") (NormalImpulse :type Vector :default "0, 0, 0") (Hit :type Hit%20Result%20Structure%20%28by%20ref%29))
  ;[1 1 1] TICK
  ;;[1 1 1] Hit
)

(event Input|ActionEvents|InputActionMouseClick
  (params (Key :type Key%20Structure :default "AnyKey"))
  ;[1 1 1] Camera
  (:Pressed
    (Variables|Default|Setinspect true))
  (:Released
    (Variables|Default|Setinspect false)))

(event Input|ActionEvents|InputActionUse
  (params (Key :type Key%20Structure :default "AnyKey"))
  (bind _skateboard (Variables|Default|Getskateboard))
  ;[1 1 1] Usables
  (:Pressed
    (if (not (Variables|Default|Getskating))
      (Utilities|IsValid _skateboard
        (:Is%20Valid
          (CallFunction|EnableSkate _skateboard))))))

(event Input|ActionEvents|InputActionGrab
  (params (Key :type Key%20Structure :default "AnyKey"))
  ;[1 1 1] Grab
  (:Pressed
    (Variables|Default|Setgrab true)
    (Variables|/Game/Blueprints/SkatingBlueprint.SkatingBlueprint_C|SetairGrab (Variables|Default|GetanimBP) true))
  (:Released
    (Variables|Default|Setgrab false)
    (Variables|/Game/Blueprints/SkatingBlueprint.SkatingBlueprint_C|SetairGrab (Variables|Default|GetanimBP) false)))

(event Input|ActionEvents|InputActionContinue
  (params (Key :type Key%20Structure :default "AnyKey"))
  ;[1 1 1] Usables
  (:Pressed
    (if (and (not (Variables|Default|Getskating)) (Variables|Default|Getragdoll))
      (CallFunction|StandUp))))

(event Input|AxisEvents|InputAxisLookUp
  (params (AxisValue :type Float%20%28single-precision%29))
  ;[1 1 1] Camera
  (Pawn|Input|AddControllerPitchInput AxisValue))

(event Input|AxisEvents|InputAxisTurn
  (params (AxisValue :type Float%20%28single-precision%29))
  ;[1 1 1] Camera
  (if (Variables|Default|Getskating)
    (if (Variables|Default|Getinspect)
      (Transformation|AddWorldRotation (Variables|Default|GetSpringArm) (Math|Vector|RotatorfromAxisandAngle (Math|Vector|GetUpVector (Variables|Default|GetCapsuleComponent)) AxisValue) false false :!label _label))
    (else
      (Pawn|Input|AddControllerYawInput AxisValue)
      (goto _label))))

(event Input|AxisEvents|InputAxisScroll
  (params (AxisValue :type Float%20%28single-precision%29))
  ;[1 1 1] Camera
  (if (Variables|Default|Getinspect)
    (Variables|Default|SetcameraZoom (+ (* AxisValue 6e+01) (Variables|Default|GetcameraZoom)))))

(event Input|AxisEvents|InputAxisMoveForward
  (params (AxisValue :type Float%20%28single-precision%29))
  ;[1 1 1] Skate Input
  (Variables|Default|SetmoveForward AxisValue)
  (if (not (Variables|Default|Getskating))
    (Pawn|Input|AddMovementInput (Math|Vector|GetForwardVector (Math|Rotator|MakeRotator 0.0 0.0 (.Yaw (Math|Rotator|BreakRotator (Pawn|GetControlRotation :!class /Script/Engine.Pawn))))) (Variables|Default|GetmoveForward) true)
    (if (> (Variables|Default|GetmoveForward) 0.0)
      (Variables|/Game/Blueprints/SkatingBlueprint.SkatingBlueprint_C|Setspeed (Variables|Default|GetanimBP) (Math|Interpolation|FInterpTo (Variables|/Game/Blueprints/SkatingBlueprint.SkatingBlueprint_C|Getspeed (Variables|Default|GetanimBP)) (Math|Vector|VectorLength (Transformation|GetVelocity)) (Variables|Default|Getdelta) 5.0))
      (else
        (Variables|/Game/Blueprints/SkatingBlueprint.SkatingBlueprint_C|Setspeed (Variables|Default|GetanimBP) (Math|Interpolation|FInterpTo (Variables|/Game/Blueprints/SkatingBlueprint.SkatingBlueprint_C|Getspeed (Variables|Default|GetanimBP)) (Math|Vector|VectorLength (Transformation|GetVelocity)) (Variables|Default|Getdelta) 1e+01))))))

(event Input|AxisEvents|InputAxisMoveRight
  (params (AxisValue :type Float%20%28single-precision%29))
  ;[1 1 1] Skate rotate
  (Variables|Default|SetmoveRight AxisValue)
  (if (Variables|Default|Getskating)
    (if (or (Variables|Default|GetinAir) (Variables|Default|Getolie_up))
      (Variables|Default|SetairRotation (+ (Variables|Default|GetairRotation) (* (Variables|Default|GetmoveRight) 1.8)))
      (else
        (Variables|Default|SetairRotation 0.0)))
    (bind _output_get (Variables|Default|SetturnRotation (Math|Vector|RotatorfromAxisandAngle (Math|Vector|GetUpVector (Variables|Character|GetMesh)) (* AxisValue 1.8))))
    (Transformation|AddWorldRotation (Variables|Default|GetCapsuleComponent) _output_get false false)
    (Variables|/Game/Blueprints/SkatingBlueprint.SkatingBlueprint_C|Setlean (Variables|Default|GetanimBP) (Math|Interpolation|FInterpTo (Variables|/Game/Blueprints/SkatingBlueprint.SkatingBlueprint_C|Getlean (Variables|Default|GetanimBP)) (* (Variables|Default|GetmoveRight) 1e+02) (Variables|Default|Getdelta) 3.0))))

(event Input|KeyboardEvents|SpaceBar
  (params (Key :type Key%20Structure :default "AnyKey"))
  ;[1 1 1] TICK
  ;;[1 1 1] Olie
  (:Pressed
    (Variables|/Game/Blueprints/SkatingBlueprint.SkatingBlueprint_C|Setolie_tab (Variables|Default|GetanimBP) 2)
    (Variables|/Game/Blueprints/SkatingBlueprint.SkatingBlueprint_C|Setolie_up (Variables|Default|GetanimBP) true))
  (:Released
    (Variables|/Game/Blueprints/SkatingBlueprint.SkatingBlueprint_C|Setolie_up (Variables|Default|GetanimBP) false)))

(event Input|KeyboardEvents|T
  (params (Key :type Key%20Structure :default "AnyKey"))
  ;[1 1 1] Usables
  (:Pressed
    (CallFunction|Fall)
    (Variables|Default|SetcurrentBlendWeight 1.0)))

(event Input|KeyboardEvents|LeftShift
  (params (Key :type Key%20Structure :default "AnyKey"))
  ;[1 1 1] Walk/Run
  (:Pressed
    (Variables|/Script/Engine.CharacterMovementComponent|SetMaxWalkSpeed (Variables|Character|GetCharacterMovement) 6e+02))
  (:Released
    (Variables|/Script/Engine.CharacterMovementComponent|SetMaxWalkSpeed (Variables|Character|GetCharacterMovement) 2e+02)))

(event Input|KeyboardEvents|W
  (params (Key :type Key%20Structure :default "AnyKey"))
  ;[1 1 1] Skate Input
  (:Pressed
    (Variables|/Game/Blueprints/SkatingBlueprint.SkatingBlueprint_C|Setpush (Variables|Default|GetanimBP) true)))

(fn ConstructionScript)

(fn ZoomCamera
  (Variables|/Script/Engine.SpringArmComponent|SetTargetArmLength (Variables|Default|GetSpringArm) (Math|Interpolation|FInterpTo (Variables|/Script/Engine.SpringArmComponent|GetTargetArmLength (Variables|Default|GetSpringArm)) (+ (Variables|Default|GetcameraOffset) (Variables|Default|GetcameraZoom)) (Variables|Default|Getdelta) 2.0)))

(fn TraceLedge
  (bind _capsulecomponent (Variables|Default|GetCapsuleComponent))
  (bind _capsulecomponent_2 (Variables|Default|GetCapsuleComponent))
  (bind _returnvalue (Math|Vector|GetForwardVector _capsulecomponent))
  (bind _returnvalue_2 (Transformation|GetWorldLocation _capsulecomponent))
  (bind _returnvalue_3 (Transformation|GetWorldLocation _capsulecomponent_2))
  (bind _returnvalue_4 (* _returnvalue -5e+02))
  (bind _returnvalue_5 (+ _returnvalue_2 _returnvalue_4))
  (bind (_x _y) (Math|Vector|BreakVector _returnvalue_5))
  ;[1 1 1] Comment
  (bind (_outhit _returnvalue_6) (Collision|BoxTraceByChannel _returnvalue_3 (+ _returnvalue_3 "0, 0,-10000.000000") "100.000000,100.000000,100.000000" "0, 0, 0" "TraceTypeQuery1" true 0 "None"))
  (if _returnvalue_6
    (bind (_outhit_2 _returnvalue_7) (Collision|LineTraceByChannel (Math|Vector|MakeVector _x _y (.Z (Math|Vector|BreakVector (.ImpactPoint (Collision|BreakHitResult _outhit))))) (.ImpactPoint (Collision|BreakHitResult _outhit)) "TraceTypeQuery1" false 0 "None" true "(R=1.000000,G=0.000000,B=0.000000,A=1.000000)" "(R=0.000000,G=1.000000,B=0.000000,A=1.000000)" 1.0))
    (if _returnvalue_7
      (Variables|Default|SetledgeNormal (.ImpactNormal (Collision|BreakHitResult _outhit_2)))
      (Rendering|Debug|DrawDebugPoint (.ImpactPoint (Collision|BreakHitResult _outhit_2)) 1e+01 "(R=0.168409,G=1.000000,B=0.000000,A=1.000000)" 1.0)))
  (if true
    _
    (else
      _))
  (return))

(fn Trace)

(fn PrintString)

(fn TraceBoard
  (Variables|Default|SethitForward false)
  (Variables|Default|SethitBackward false)
  (bind (_hit _impactnormal) (Class|SkateCharacter|LineTraceDown -1e+02 -35.0 (Variables|Default|Getskateboard)))
  (Variables|Default|SethitForward _hit)
  (Variables|Default|SetforwardNormal _impactnormal)
  (bind (_hit_2 _impactnormal_2) (Class|SkateCharacter|LineTraceDown -1e+02 35.0 (Variables|Default|Getskateboard)))
  (Variables|Default|SethitBackward _hit_2)
  (Variables|Default|SetbackwardNormal _impactnormal_2))

(fn TraceGround
  (bind (_hit _impactnormal _impactpoint) (Class|SkateCharacter|CapsuleTraceDown 4e+01 96.0 (Variables|Default|Getskateboard)))
  (if _hit
    (Variables|Default|SetinAir false)
    (Variables|Default|SetsurfaceNormal _impactnormal)
    (Variables|Default|SetsurfacePosition _impactpoint)
    (else
      (Variables|Default|SetinAir true))))

(fn Fall
  (bind _skateboard (Variables|Default|Getskateboard))
  (Variables|Default|Setskating false)
  (Variables|Default|Setragdoll true)
  (Variables|/Game/Blueprints/SkatingBlueprint.SkatingBlueprint_C|Setskating (Variables|Default|GetanimBP) false)
  (Variables|/Game/Blueprints/SkatingBlueprint.SkatingBlueprint_C|SetgetUp (Variables|Default|GetanimBP) false)
  (Variables|/Game/Blueprints/SkatingBlueprint.SkatingBlueprint_C|Setragdoll (Variables|Default|GetanimBP) true)
  (Utilities|FlowControl|Sequence
    (:then_0
      (Transformation|DetachFromActor _skateboard "KeepRelative" "KeepRelative" "KeepRelative")
      (Default|OnLeft _skateboard))
    (:then_1
      (Transformation|DetachFromComponent (Variables|Character|GetMesh) "KeepWorld" "KeepWorld" "KeepWorld" false)
      (Class|SkeletalMeshComponent|SetAllBodiesBelowSimulatePhysics (Variables|Character|GetMesh) (Utilities|Name|MakeLiteralName "CC_Base_Hip") true true)
      (Variables|/Script/Engine.MovementComponent|SetVelocity (Variables|Default|GetFloatingPawnMovement) "0, 0, 0"))))

(fn CorrectRagdoll
  (bind _mesh (Variables|Character|GetMesh))
  (bind _returnvalue (Transformation|GetSocketLocation _mesh "CC_Base_Hip"))
  (bind (_outhit _returnvalue_2) (Collision|LineTraceByChannel (+ _returnvalue "0, 0,200.000000") (+ _returnvalue "0, 0,-200.000000") "TraceTypeQuery1" true 0 "None"))
  (if _returnvalue_2
    (Transformation|SetWorldLocation (Variables|Default|GetCapsuleComponent) (+ (.ImpactPoint (Collision|BreakHitResult _outhit)) "0, 0,96.000000") false false)
    (Transformation|SetWorldRotation (Variables|Default|GetCapsuleComponent) (Math|Rotator|MakeRotator 0.0 0.0 (.Yaw (Math|Rotator|BreakRotator (Transformation|GetWorldRotation (Variables|Character|GetMesh))))) false false)))

(fn StandUpRagdoll
  (if (> (Variables|Default|GetcurrentBlendWeight) 0.0)
    (Class|SkeletalMeshComponent|SetAllBodiesBelowPhysicsBlendWeight (Variables|Character|GetMesh) (Utilities|Name|MakeLiteralName "CC_Base_Hip") 1.0 false true)
    (Variables|Default|SetcurrentBlendWeight (Math|Interpolation|FInterpTo (Variables|Default|GetcurrentBlendWeight) 0.0 (Variables|Default|Getdelta) 1.0))
    (bind _output_get (LocalVariables|SetcurrentWeight (Math|Interpolation|FInterpTo (Variables|Default|GetcurrentBlendWeight) 0.0 (Variables|Default|Getdelta) 1.0)))
    (if (== _output_get 0.0)
      _)))

(fn StandUp
  (bind _mesh (Variables|Character|GetMesh))
  (bind _returnvalue (Transformation|GetSocketLocation _mesh "CC_Base_Hip"))
  (bind _returnvalue_2 (Collision|LineTraceByChannel _returnvalue (+ _returnvalue (* (Math|Vector|GetForwardVector (Variables|Character|GetMesh)) 2e+03)) "TraceTypeQuery1" true 0 "Persistent"))
  (Variables|/Game/Blueprints/SkatingBlueprint.SkatingBlueprint_C|SetgetUpFromUp (Variables|Default|GetanimBP) _returnvalue_2)
  (Variables|Default|Setragdoll false)
  (Variables|/Game/Blueprints/SkatingBlueprint.SkatingBlueprint_C|SetgetUp (Variables|Default|GetanimBP) true)
  (Variables|/Game/Blueprints/SkatingBlueprint.SkatingBlueprint_C|Setragdoll (Variables|Default|GetanimBP) false)
  (Transformation|AttachComponentToComponent (Variables|Character|GetMesh) (Variables|Default|GetCapsuleComponent) "None" "KeepRelative" "KeepWorld" "KeepRelative" true)
  (Transformation|SetRelativeLocationAndRotation (Variables|Character|GetMesh) "0, 0,-96.000000" "0.000000,-90.000000,0.000000" false false)
  (Transformation|AddWorldRotation (Variables|Default|GetCapsuleComponent) "0,90.000000, 0" false false)
  (Components|Activation|Deactivate (Variables|Default|GetFloatingPawnMovement))
  (Components|Activation|Activate (Variables|Character|GetCharacterMovement) true))

(fn EnableSkate
  (params (base :type Base%20Object%20Reference))
  (bind _skateboard_base1 (Variables|/Game/Blueprints/Base.Base_C|Getskateboard_base1 base))
  (Collision|SetActorEnableCollision base false)
  (Physics|SetSimulatePhysics _skateboard_base1 false)
  (Transformation|AttachComponentToComponent _skateboard_base1 (Variables|Character|GetMesh) "skateboard_rootnode" "SnapToTarget" "SnapToTarget" "SnapToTarget" false)
  (Transformation|SetRelativeLocationAndRotation _skateboard_base1 "0, 0,0.000000" "0.000000,0.000000,0.000000" false false)
  (Utilities|FlowControl|Sequence
    (:then_0
      (Components|Activation|SetActive (Variables|Default|GetFloatingPawnMovement) true false)
      (Components|Activation|Deactivate (Variables|Character|GetCharacterMovement))
      (Default|OnUsed (Variables|Default|Getskateboard)))
    (:then_1
      (Variables|/Game/Blueprints/SkatingBlueprint.SkatingBlueprint_C|Setskating (Variables|Default|GetanimBP) true)
      (Variables|Default|Setskating true))))

(fn SpawnSkateboard
  (bind _returnvalue (Game|SpawnActorfromClass "/Game/Blueprints/Base.Base_C" (Math|Transform|MakeTransform "0, 0, 0") "AlwaysSpawn" 0 true 0))
  (bind _output_get (Variables|Default|Setskateboard _returnvalue))
  (Default|OnUsed _output_get)
  (Transformation|AttachComponentToComponent (Variables|/Game/Blueprints/Base.Base_C|Getskateboard_base1 _output_get) (Variables|Character|GetMesh) "skateboard_rootnode" "SnapToTarget" "SnapToTarget" "SnapToTarget" true))

(fn GetGroundDistance
  (bind _returnvalue (Transformation|GetActorLocation))
  (bind _outhit (Collision|LineTraceByChannel _returnvalue (+ _returnvalue "0,0.000000,2000.000000") "TraceTypeQuery1" true 0 "None"))
  (return (.Z (Math|Vector|BreakVector (- (Transformation|GetActorLocation) (.ImpactPoint (Collision|BreakHitResult _outhit)))))))